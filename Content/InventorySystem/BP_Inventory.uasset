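; BP_Inventory stores items and their quantities in a map, with functions to add, subtract and remove them.
; AddItem stacks amounts but only while the entry count is below InvenMaxCount, so a full inventory also rejects existing items.
; SubtractItem lowers the count or calls RemoveItem on an exact match, ignoring larger amounts.
; Successful changes broadcast the map through OnInventroyUpdate, with debug prints on add and partial subtract.
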(fn `Add Item`
  (params (`New Item` :type "/Game/Blueprints/Items/PDA_Item Object Reference") (`Add Amount` :type Integer))
  (bind _inventory (`self.Inventory`))
  (`/Engine/EditorBlueprintResources/StandardMacros.IsValid` `New Item`
    (:`Is Valid`
      (if (> (`self.Inven Max Count`) (`BlueprintMapLibrary.Map_Length` (`self.Inventory`)))
        (`BlueprintMapLibrary.Map_Add` _inventory `New Item` (+ (`BlueprintMapLibrary.Map_Find` _inventory `New Item`) `Add Amount`))
        (`KismetSystemLibrary.PrintString` null (`KismetStringLibrary.Concat_StrStr` "Add Item : " (`KismetTextLibrary.Conv_TextToString` (`/Game/Blueprints/Items/PDA_Item.Item Name` `New Item`))))
        (`self.On Inventroy Update` (`self.Inventory`))))))

(fn `Remove Item`
  (params (`Remove Item` :type "/Game/Blueprints/Items/PDA_Item Object Reference"))
  (bind _returnvalue (`BlueprintMapLibrary.Map_Remove` (`self.Inventory`) `Remove Item`))
  (if _returnvalue
    (`self.On Inventroy Update` (`self.Inventory`))))

(fn `Subtract Item`
  (params (`Target Item` :type "/Game/Blueprints/Items/PDA_Item Object Reference") (`Subtract Amount` :type Integer))
  (bind _inventory (`self.Inventory`))
  (bind _value (`BlueprintMapLibrary.Map_Find` _inventory))
  (`/Engine/EditorBlueprintResources/StandardMacros.IsValid` `Target Item`
    (:`Is Valid`
      (if (> _value `Subtract Amount`)
        (`BlueprintMapLibrary.Map_Add` _inventory null (- _value `Subtract Amount`))
        (`KismetSystemLibrary.PrintString` null (`KismetStringLibrary.Concat_StrStr` "Subtract Item : " (`KismetTextLibrary.Conv_TextToString` (`/Game/Blueprints/Items/PDA_Item.Item Name` `Target Item`))))
        (`self.On Inventroy Update` (`self.Inventory`))
        (elif (== _value `Subtract Amount`)
          (`self.Remove Item` `Target Item`))))))