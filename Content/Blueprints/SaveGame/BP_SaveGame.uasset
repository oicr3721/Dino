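; BP_SaveGame holds the player's data plus inventory and quick slot contents, converting between live objects and saved data.
; SaveGameData flattens item references into ItemID-keyed counts and slot-to-ID pairs, marking empty slots "None", inside an InvenData struct.
; LoadInvenData resolves those IDs through ItemDict, then constructs new BP_ItemInventory and BP_QuickSlot objects with their saved limits.
; Unresolved IDs are dropped from the inventory but kept as empty quick slots.
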(fn `Load Inven Data`
  (params (`Game Instance` :type "/Game/GI_GameInstance Object Reference"))
  (returns (`item inven` :type "/Game/Blueprints/Inven/BP_ItemInventory Object Reference") (`quick slot` :type "/Game/Blueprints/Inven/BP_QuickSlot Object Reference"))
  (locals (`Inven Contents` :type "Map of /Game/Blueprints/Items/PDA_Item Object Reference to Object Object Reference") (`QuickSlot Contents` :type "Map of Integer to /Game/Blueprints/Items/PDA_Item Object Reference"))
  (bind (_invenitems _invenmaxcount _quickslotitems) (break `/Game/Blueprints/SaveGame/S_InvenData` (`self.Inven Data`)))
  (bind (_invenitems_2 _invenmaxcount_2 _quickslotitems_2 _quickslotmaxlength) (break `/Game/Blueprints/SaveGame/S_InvenData` (`self.Inven Data`)))
  (`|ExecutionSequence`
    (:`then_0`
      ; Load Items
      (`|ExecutionSequence`
        (:`then_0`
          (bind (_keypin _valuepin) (`|MapForEach` _invenitems)
            (:`then`
              (bind (_item _find_success) (`/Game/Blueprints/Items/PDA_ItemDict.Find Item` (`self.Item Dict`) _keypin))
              (if _find_success
                (`BlueprintMapLibrary.Map_Add` (`local.Inven Contents`) _item _valuepin)))))
        (:`then_1`
          (bind (_keypin_2 _valuepin_2) (`|MapForEach` _quickslotitems)
            (:`then`
              (bind (_item_2 _find_success_2) (`/Game/Blueprints/Items/PDA_ItemDict.Find Item` (`self.Item Dict`) _valuepin_2))
              (if _find_success_2
                (`BlueprintMapLibrary.Map_Add` (`local.QuickSlot Contents`) _keypin_2 _item_2)
                (else
                  (`BlueprintMapLibrary.Map_Add` (`local.QuickSlot Contents`) _keypin_2))))))))
    (:`then_1`
      ; Create Inven Objects
      (bind _returnvalue (`|GenericCreateObject` `Game Instance` "/Game/Blueprints/Inven/BP_ItemInventory.BP_ItemInventory_C" (`local.Inven Contents`) _invenmaxcount_2))
      (bind _returnvalue_2 (`|GenericCreateObject` `Game Instance` "/Game/Blueprints/Inven/BP_QuickSlot.BP_QuickSlot_C" (`local.QuickSlot Contents`) _quickslotmaxlength 1))
      (return _returnvalue _returnvalue_2))))

(fn `Save Game Data`
  (params (`Item Inven` :type "/Game/Blueprints/Inven/BP_ItemInventory Object Reference") (`Quick Slot Inven` :type "/Game/Blueprints/Inven/BP_QuickSlot Object Reference") (`Player Data` :type "/Game/Blueprints/SaveGame/S_PlayerData Structure"))
  (locals (`Inven Save` :type "Map of Name to Integer") (`Quick Slot Save` :type "Map of Integer to Name"))
  (`|ExecutionSequence`
    (:`then_0`
      (bind (_keypin _valuepin) (`|MapForEach` (`/Game/Blueprints/Inven/BP_ItemInventory.Contents` `Item Inven`))
        (:`then`
          (`BlueprintMapLibrary.Map_Add` (`local.Inven Save`) (`/Game/Blueprints/Items/PDA_Item.Item ID` _keypin) _valuepin))))
    (:`then_1`
      (bind (_keypin_2 _valuepin_2) (`|MapForEach` (`/Game/Blueprints/Inven/BP_QuickSlot.Slot Contents` `Quick Slot Inven`))
        (:`then`
          (`/Engine/EditorBlueprintResources/StandardMacros.IsValid` _valuepin_2
            (:`Is Valid`
              (`BlueprintMapLibrary.Map_Add` (`local.Quick Slot Save`) _keypin_2 (`/Game/Blueprints/Items/PDA_Item.Item ID` _valuepin_2)))
            (:`Is Not Valid`
              (`BlueprintMapLibrary.Map_Add` (`local.Quick Slot Save`) _keypin_2))))))
    (:`then_2`
      (set `self.Player Data` `Player Data`)
      (set `self.Inven Data` (make `/Game/Blueprints/SaveGame/S_InvenData` (`local.Inven Save`) (`/Game/Blueprints/Inven/BP_ItemInventory.Max Item Count` `Item Inven`) (`local.Quick Slot Save`) (`/Game/Blueprints/Inven/BP_QuickSlot.Max Length` `Quick Slot Inven`))))))