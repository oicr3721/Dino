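; Breakable rock actor that can slide between two locations and shatter on demand.
; MoveTo runs a timeline that lerps the actor from a start to a target location without sweeping.
; Break enables physics on the rock component, then spawns and triggers a short-lived, self-destroying FS_MasterField at its location to apply the fracturing field.
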(event `Move To`
  (params (`Start Location` :type "Vector Structure") (`Target Location` :type "Vector Structure"))
  (bind (_direction _timeline_float) (`Timeline|Move Timeline` :!via `PlayFromStart`)
    (:`Update`
      (`self.K2_SetActorLocation` (`KismetMathLibrary.VLerp` `Start Location` `Target Location` _timeline_float)))))

(fn `Break`
  (`PrimitiveComponent.SetSimulatePhysics` (`self.GC_BP_RockToBreak`) true)
  (bind _returnvalue (`|SpawnActorFromClass` "/Engine/EditorResources/FieldNodes/FS_MasterField.FS_MasterField_C" (`KismetMathLibrary.Conv_VectorToTransform` (`SceneComponent.K2_GetComponentLocation` (`self.GC_BP_RockToBreak`))) "Undefined" "MultiplyWithRoot" null null))
  (set `/Engine/EditorResources/FieldNodes/FS_MasterField.ActivationType` "NewEnumerator4" _returnvalue)
  (set `/Engine/EditorResources/FieldNodes/FS_MasterField.DestroyActor` true _returnvalue)
  (set `/Engine/EditorResources/FieldNodes/FS_MasterField.UseLifespan` true _returnvalue)
  (set `/Engine/EditorResources/FieldNodes/FS_MasterField.FieldLifespan` 0.01 _returnvalue)
  (set `/Engine/EditorResources/FieldNodes/FS_MasterField.Radial Magnitude` 1.0 _returnvalue)
  (`/Engine/EditorResources/FieldNodes/FS_MasterField.CE_Trigger` _returnvalue))

(fn `UserConstructionScript`)