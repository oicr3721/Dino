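; BP_Text is a placeable world text actor that displays an editable Text variable through a TextRender component.
; The construction script applies the Text to the TextRender.
; At BeginPlay it compares both values as strings and sets the component text again only if they differ.
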(event `self.ReceiveBeginPlay`
  (if (`KismetStringLibrary.NotEqual_StrStr` (`KismetTextLibrary.Conv_TextToString` (`TextRenderComponent.Text` (`self.TextRender`))) (`KismetTextLibrary.Conv_TextToString` (`self.Text`)))
    (`TextRenderComponent.K2_SetText` (`self.TextRender`) (`self.Text`))))

(fn `UserConstructionScript`
  (`TextRenderComponent.K2_SetText` (`self.TextRender`) (`self.Text`)))