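; BP_Gate is an interactable gate object that sends the player to another level.
; It is always interactable and reports its InteractionName through the interaction functions.
; On Interact it gets the BP_FirstPersonGameMode and, if its LevelTransition is valid, calls MoveToLevel with the gate's LevelName.
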(event `/Game/Blueprints/Objects/BPI_Interact.Interact`
  (bind _asbp_first_person_game_mode (cast `/Game/FirstPerson/Blueprints/BP_FirstPersonGameMode` (`GameplayStatics.GetGameMode`)))
  (bind _level_transition (`/Game/FirstPerson/Blueprints/BP_FirstPersonGameMode.Level Transition` _asbp_first_person_game_mode))
  (`/Engine/EditorBlueprintResources/StandardMacros.IsValid` _level_transition
    (:`Is Valid`
      (`/Game/Blueprints/BP_LevelTransitionManager.Move To Level` _level_transition (`self.Level Name`)))))

(fn `Get Interaction Name`
  (returns (`Interaction Name` :type Text))
  (return (`self.Interaction Name`)))

(fn `Is Interactable`
  (returns (Interactable :type Boolean))
  (return true))

(fn `UserConstructionScript`)