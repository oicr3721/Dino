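; BP_StoreItem is an interactable shop item that the player buys with money.
; Its interaction prompt is built from the name and price in ItemData.
; On Interact it checks PlayerMoney in GI_GameInstance, deducts the price, adds one of the item through the game instance and destroys itself.
; When funds are short, it only prints a refusal message.
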(event `/Game/Blueprints/Objects/BPI_Interact.Interact`
  (params (Player :type "/Game/FirstPerson/Blueprints/BP_FirstPersonCharacter Object Reference"))
  (bind _price (`/Game/Blueprints/Items/PDA_Item.Price` (`self.Item Data`)))
  (bind _asgi_game_instance (cast `/Game/GI_GameInstance` (`GameplayStatics.GetGameInstance`)))
  (bind _player_money (`/Game/GI_GameInstance.Player Money` _asgi_game_instance))
  (if (>= _player_money _price)
    (set `/Game/GI_GameInstance.Player Money` (- _player_money _price) _asgi_game_instance)
    (`/Game/GI_GameInstance.Add Item` _asgi_game_instance (`self.Item Data`) 1)
    (`self.K2_DestroyActor`)
    (else
      (`KismetSystemLibrary.PrintString` "You can't buy this."))))

(fn `Get Interaction Name`
  (returns (`Interaction Name` :type Text))
  (return (`KismetTextLibrary.Conv_StringToText` (`KismetStringLibrary.Concat_StrStr` "Buy " (`KismetTextLibrary.Conv_TextToString` (`/Game/Blueprints/Items/PDA_Item.Item Name` (`self.Item Data`))) " : " (`KismetStringLibrary.Conv_IntToString` (`/Game/Blueprints/Items/PDA_Item.Price` (`self.Item Data`))) "G"))))

(fn `Is Interactable`
  (returns (Interactable :type Boolean))
  (return true))

(fn `UserConstructionScript`
  (`parent.UserConstructionScript`))