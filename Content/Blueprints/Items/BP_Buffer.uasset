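; BP_Buffer is an always-interactable item that grants a temporary buff or debuff to the player who interacts with it.
; On Interact it casts its ItemData to PDA_Food and passes that data asset's stat modifier (speed, power and duration) to the player's AttachBuffDebuff.
; Items without valid food data do nothing, and the item is neither consumed nor destroyed here.
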(event `/Game/Blueprints/Objects/BPI_Interact.Interact`
  (params (Player :type "/Game/Blueprints/Characters/BP_PlayerCharacter Object Reference"))
  (bind _aspda_food (cast `/Game/Blueprints/Items/PDA_Food` (`self.Item Data`)))
  (`/Engine/EditorBlueprintResources/StandardMacros.IsValid` _aspda_food
    (:`Is Valid`
      (bind (_playerspeedmultiplier _playerpowermultiplier _playereffectduration) (break `/Game/Blueprints/Items/S_ItemEffect` (`/Game/Blueprints/Items/PDA_Food.Stat Modifier` _aspda_food)))
      (`/Game/Blueprints/Characters/BP_Digger.Attach Buff Debuff` Player _playerspeedmultiplier _playerpowermultiplier _playereffectduration))))

(fn `Is Interactable`
  (params (Player :type "/Game/Blueprints/Characters/BP_PlayerCharacter Object Reference"))
  (returns (Interactable :type Boolean))
  (return true))

(fn `UserConstructionScript`
  (`parent.UserConstructionScript`))