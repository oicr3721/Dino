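; Item lying in voxel terrain that is always interactable under the "Get" prompt and digs a hole in the ground when picked up.
; Interact sphere-traces at the item mesh to find the VoxelWorld, removes a sphere just below the hit surface and smooths a wider area around it.
; GetItem then completes the pickup, which only happens if the trace hit a VoxelWorld.
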(event `self.ReceiveBeginPlay`
  (`parent.ReceiveBeginPlay`))

(event `/Game/Blueprints/Objects/BPI_Interact.Interact`
  (params (Player :type "/Game/FirstPerson/Blueprints/BP_FirstPersonCharacter Object Reference"))
  (bind _returnvalue (`SceneComponent.K2_GetComponentLocation` (`self.Item Mesh`)))
  (bind _outhit (`KismetSystemLibrary.SphereTraceSingle` :`Start` _returnvalue :`End` _returnvalue :`Radius` 30.0 :`TraceChannel` "TraceTypeQuery3" :`DrawTime` 1.0))
  (bind (_bblockinghit _binitialoverlap _time _distance _location _impactpoint _normal _impactnormal _physmat _hitactor) (`GameplayStatics.BreakHitResult` _outhit))
  (bind _asvoxel_world (cast `VoxelWorld` _hitactor))
  (bind _returnvalue_2 (- _impactpoint (* _normal (10.0 10.0 10.0))))
  (`VoxelSphereTools.RemoveSphere` _asvoxel_world _returnvalue_2 35.0)
  (`VoxelSphereTools.SmoothSphere` _asvoxel_world _returnvalue_2 50.0 80.0 1 "Tip")
  (`self.Get Item`))

(fn `Get Interaction Name`
  (returns (`Interaction Name` :type Text))
  (return "Get"))

(fn `Is Interactable`
  (returns (Interactable :type Boolean))
  (return true))

(fn `UserConstructionScript`
  (`parent.UserConstructionScript`))