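; PDA_Shovel is a shovel item that modifies the player's digging radius and walk speed while equipped.
; Equip multiplies DigRadius by PowerMultiplier and the character movement's MaxWalkSpeed by SpeedMultiplier.
; Unequip divides by the same multipliers to undo the change, editing the live values in place rather than caching the originals.
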(event `/Game/Blueprints/Items/BPI_Equippable.Equip`
  (params (Player :type "/Game/Blueprints/Characters/BP_PlayerCharacter Object Reference"))
  (bind _charactermovement (`Character.CharacterMovement` Player))
  (set `/Game/Blueprints/Characters/BP_Digger.Dig Radius` (* (`/Game/Blueprints/Characters/BP_Digger.Dig Radius` Player) (`self.Power Multiplier`)) Player)
  (set `CharacterMovementComponent.MaxWalkSpeed` (* (`CharacterMovementComponent.MaxWalkSpeed` _charactermovement) (`self.Speed Multiplier`)) _charactermovement))

(event `/Game/Blueprints/Items/BPI_Equippable.Unequip`
  (params (Player :type "/Game/Blueprints/Characters/BP_PlayerCharacter Object Reference"))
  (bind _charactermovement (`Character.CharacterMovement` Player))
  (set `/Game/Blueprints/Characters/BP_Digger.Dig Radius` (/ (`/Game/Blueprints/Characters/BP_Digger.Dig Radius` Player) (`self.Power Multiplier`)) Player)
  (set `CharacterMovementComponent.MaxWalkSpeed` (/ (`CharacterMovementComponent.MaxWalkSpeed` _charactermovement) (`self.Speed Multiplier`)) _charactermovement))