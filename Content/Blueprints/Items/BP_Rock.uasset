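; BP_Rock is an interactable rock pickup whose mesh is set from its RockInfo data at construction.
; On interaction it adds RockInfo to the game instance's rock inventory and, if that succeeds, digs around itself and is destroyed.
; Digging sphere-traces at the rock's location to find the VoxelWorld, then removes and smooths a sphere just beneath the hit surface, leaving a hollow in the terrain.
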(event `/Game/Blueprints/Objects/BPI_Interact.Interact`
  (params (Player :type "/Game/Blueprints/Characters/BP_PlayerCharacter Object Reference"))
  (bind _asgi_game_instance (cast `/Game/GI_GameInstance` (`GameplayStatics.GetGameInstance`)))
  (bind _add_success (`/Game/Blueprints/Inven/BP_RockInventory.Add` (`/Game/GI_GameInstance.Rock Inven` _asgi_game_instance) (`self.Rock Info`)))
  (if _add_success
    (`self.Dig Around`)
    (`self.K2_DestroyActor`)))

(fn `Dig Around`
  (bind _returnvalue (`SceneComponent.K2_GetComponentLocation` (`self.StaticMesh`)))
  (bind _outhit (`KismetSystemLibrary.SphereTraceSingle` :`Start` _returnvalue :`End` _returnvalue :`Radius` 30.0 :`TraceChannel` "TraceTypeQuery3" :`DrawTime` 1.0))
  (bind (_bblockinghit _binitialoverlap _time _distance _location _impactpoint _normal _impactnormal _physmat _hitactor) (`GameplayStatics.BreakHitResult` _outhit))
  (bind _asvoxel_world (cast `VoxelWorld` _hitactor))
  (bind _returnvalue_2 (- _impactpoint (* _normal (10.0 10.0 10.0))))
  (`VoxelSphereTools.RemoveSphere` _asvoxel_world _returnvalue_2 35.0)
  (`VoxelSphereTools.SmoothSphere` _asvoxel_world _returnvalue_2 50.0 80.0 1 "Tip"))

(fn `Get Interaction Name`
  (params (Player :type "/Game/Blueprints/Characters/BP_PlayerCharacter Object Reference"))
  (returns (`Interaction Name` :type Text))
  (return "Get"))

(fn `Is Interactable`
  (params (Player :type "/Game/Blueprints/Characters/BP_PlayerCharacter Object Reference"))
  (returns (Interactable :type Boolean))
  (return true))

(fn `UserConstructionScript`
  (bind (_fossilprob _charmprob _etcprob _birthfloor _rockmesh) (break `/Game/Blueprints/Items/S_RockInfo` (`self.Rock Info`)))
  (`/Engine/EditorBlueprintResources/StandardMacros.IsValid` _rockmesh
    (:`Is Valid`
      (`StaticMeshComponent.SetStaticMesh` (`self.StaticMesh`) _rockmesh))))