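; BP_WorldItem is a pickup actor that displays an item in the world and, on interaction, adds it to the GI_GameInstance inventory and destroys itself.
; The construction script instantiates an item object from the chosen ItemType class, recreating it when the class changes.
; UpdateItemMesh applies that object's mesh and scale and enables physics, async-loading the soft mesh reference first if it is not yet loaded.
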(event `Load Item Mesh`
  (params (`Soft Ref` :type "StaticMesh Soft Object Reference"))
  (`|LoadAsset` `Soft Ref`
    (:`Completed`
      (`self.Update Item Mesh`))))

(event `/Game/Blueprints/Objects/BPI_Interact.Interact`
  (`self.Get Item`))

(event `self.ReceiveBeginPlay`
  (`self.Update Item Mesh`))

(fn `Get Interaction Name`
  (returns (`Interaction Name` :type Text))
  (return "Get"))

(fn `Get Item`
  (bind _asgi_game_instance (cast `/Game/GI_GameInstance` (`GameplayStatics.GetGameInstance`)))
  (`/Game/GI_GameInstance.Add Item` _asgi_game_instance (`self.Item Object`))
  (`self.K2_DestroyActor`))

(fn `Is Interactable`
  (returns (Interactable :type Boolean))
  (return true))

(fn `Update Item Mesh`
  (bind _item_object (`self.Item Object`)
    (:`then`
      (bind _item_mesh (`/Game/Blueprints/Items/ItemBase.Item Mesh` _item_object))
      (bind _output (`|ConvertAsset` _item_mesh))
      (`/Engine/EditorBlueprintResources/StandardMacros.IsValid` _output
        (:`Is Valid`
          (`StaticMeshComponent.SetStaticMesh` (`self.Item Mesh`) _output)
          (`SceneComponent.SetWorldScale3D` (`self.Item Mesh`) (`/Game/Blueprints/Items/ItemBase.Mesh Scale` (`self.Item Object`)))
          (`PrimitiveComponent.SetSimulatePhysics` (`self.Item Mesh`) true))
        (:`Is Not Valid`
          (`self.Load Item Mesh` _item_mesh))))
    (:`else`
      (`StaticMeshComponent.SetStaticMesh` (`self.Item Mesh`) null))))

(fn `UserConstructionScript`
  (`self.Item Type`
    (:`then`
      (bind _item_object (`self.Item Object`)
        (:`then`
          (if (not (== (`self.Item Type`) (`GameplayStatics.GetObjectClass` _item_object)))
            (bind _returnvalue (`|GenericCreateObject` (`self.Item Type`) :!label _label))
            (set `self.Item Object` _returnvalue)))
        (:`else`
          (goto _label)))
      (`self.Update Item Mesh`))
    (:`else`)))