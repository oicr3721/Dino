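; BP_Speed_BuffDebuff is a timed speed buff or debuff actor that changes the movement speed of the character it is attached to.
; After a short delay on BeginPlay, it multiplies the parent character's MaxWalkSpeed by SpeedMultiplier and sets its lifespan to Duration.
; On EndPlay it divides MaxWalkSpeed by the same multiplier to undo the change, relying on still being attached to that character.
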(event `self.ReceiveBeginPlay`
  (`KismetSystemLibrary.Delay` 0.2)
  (bind _ascharacter (cast `Character` (`self.GetAttachParentActor`)))
  (bind _charactermovement (`Character.CharacterMovement` _ascharacter))
  (set `CharacterMovementComponent.MaxWalkSpeed` (* (`CharacterMovementComponent.MaxWalkSpeed` _charactermovement) (`self.Speed Multiplier`)) _charactermovement)
  (`self.SetLifeSpan` (`self.Duration`)))

(event `self.ReceiveEndPlay`
  (params (EndPlayReason :type "EEndPlayReason Enum" :default "Destroyed"))
  (bind _ascharacter (cast `Character` (`self.GetAttachParentActor`)))
  (bind _charactermovement (`Character.CharacterMovement` _ascharacter))
  (set `CharacterMovementComponent.MaxWalkSpeed` (/ (`CharacterMovementComponent.MaxWalkSpeed` _charactermovement) (`self.Speed Multiplier`)) _charactermovement))

(fn `UserConstructionScript`)