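; BP_Power_BuffDebuff is a timed power modifier that scales the dig radius of the BP_Digger it is attached to.
; Shortly after BeginPlay it multiplies the parent's DigRadius by PowerMultiplier and sets its own lifespan to Duration.
; EndPlay divides by the same multiplier to undo the change, so one actor can serve as either buff or debuff.
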(event `self.ReceiveBeginPlay`
  (`KismetSystemLibrary.Delay` 0.2)
  (bind _asbp_digger (cast `/Game/Blueprints/Characters/BP_Digger` (`self.GetAttachParentActor`)))
  (set `/Game/Blueprints/Characters/BP_Digger.Dig Radius` (* (`/Game/Blueprints/Characters/BP_Digger.Dig Radius` _asbp_digger) (`self.Power Multiplier`)) _asbp_digger)
  (`self.SetLifeSpan` (`self.Duration`)))

(event `self.ReceiveEndPlay`
  (params (EndPlayReason :type "EEndPlayReason Enum" :default "Destroyed"))
  (bind _asbp_digger (cast `/Game/Blueprints/Characters/BP_Digger` (`self.GetAttachParentActor`)))
  (set `/Game/Blueprints/Characters/BP_Digger.Dig Radius` (/ (`/Game/Blueprints/Characters/BP_Digger.Dig Radius` _asbp_digger) (`self.Power Multiplier`)) _asbp_digger))

(fn `UserConstructionScript`)