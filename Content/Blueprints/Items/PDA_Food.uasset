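; PDA_Food is a food item definition whose Use function applies a buff or debuff to whoever consumes it.
; It casts the user to BP_PlayerCharacter, then BP_Dog, attaching the matching player or dog effect from StatModifier.
; The player plays an eat montage, while the dog plays an idle playing montage.
; Use returns true for either character type and false for any other user.
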(fn `Use`
  (params (User :type "/Game/Blueprints/Characters/BP_Digger Object Reference"))
  (returns (UseSuccess :type Boolean))
  (bind _asbp_player_character (cast `/Game/Blueprints/Characters/BP_PlayerCharacter` User)
    (:`then`
      (`/Game/Blueprints/Characters/BP_Digger.Attach Buff Debuff` User (`.PlayerBuffDebuff_34_C38342854B487C0930686F8B3F2444E7` (break `/Game/Blueprints/Items/S_ItemEffect` (`self.Stat Modifier`))))
      (`Character.PlayAnimMontage` _asbp_player_character "/Game/Anim/Player/Eat_Montage.Eat_Montage" 1.0 "None"))
    (:`CastFailed`
      (bind _asbp_dog (cast `/Game/Blueprints/Characters/BP_Dog` User)
        (:`then`
          (`/Game/Blueprints/Characters/BP_Digger.Attach Buff Debuff` _asbp_dog (`.DogBuffDebuff_32_B531E6664417DA3C9A8A8685017E438D` (break `/Game/Blueprints/Items/S_ItemEffect` (`self.Stat Modifier`))))
          (`Character.PlayAnimMontage` _asbp_dog "/Game/German_Shepherd_3D_Model/Animations/A_type1_Idle_Playing_v01_Montage.A_type1_Idle_Playing_v01_Montage" 1.0 "None"))
        (:`CastFailed`
          (return false)))))
  (return true))