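; Timed buff/debuff actor that attaches to a BP_Digger and scales its walk speed and dig radius.
; After a short BeginPlay delay it applies the BuffDebuffData multipliers, sets its lifespan and registers in ActiveBuffDebuffs.
; EndPlay unregisters it, applies any death penalty and runs the removal math, which receives zero instead of the stored multipliers.
; ReturnRemainBuffDebuffData packages the effect with its remaining lifespan.
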(event `self.ReceiveBeginPlay`
  (bind (_speedmultiplier _powermultiplier _duration) (break `/Game/Blueprints/Items/S_BuffDebuffData` (`self.BuffDebuff Data`)))
  (`KismetSystemLibrary.Delay` 0.2)
  (bind _asbp_digger (cast `/Game/Blueprints/Characters/BP_Digger` (`self.GetAttachParentActor`)))
  (`self.Set Speed BuffDebuff` _asbp_digger _speedmultiplier)
  (`self.Set Power BuffDebuff` _asbp_digger _powermultiplier)
  (`self.SetLifeSpan` _duration)
  (`KismetArrayLibrary.Array_Add` (`/Game/Blueprints/Characters/BP_Digger.Active BuffDebuffs` _asbp_digger) self))

(event `self.ReceiveEndPlay`
  (params (EndPlayReason :type "EEndPlayReason Enum" :default "Destroyed"))
  (bind _asbp_digger (cast `/Game/Blueprints/Characters/BP_Digger` (`self.GetAttachParentActor`)))
  (`self.Remove Speed BuffDebuff` 0.0 _asbp_digger)
  (`self.Remove Power BuffDebuff` 0.0 _asbp_digger)
  (`KismetArrayLibrary.Array_RemoveItem` (`/Game/Blueprints/Characters/BP_Digger.Active BuffDebuffs` _asbp_digger) self)
  (if (`.DeathPenalty_8_1014B6F7407079813687C796F5CDD5BB` (break `/Game/Blueprints/Items/S_BuffDebuffData` (`self.BuffDebuff Data`)))
    (`/Game/Blueprints/Characters/BP_Digger.Apply Penalty` _asbp_digger)))

(fn `Remove Power BuffDebuff`
  (params (`power multiplier` :type "Float (double-precision)") (`target digger` :type "/Game/Blueprints/Characters/BP_Digger Object Reference"))
  (set `/Game/Blueprints/Characters/BP_Digger.Dig Radius` (/ `power multiplier` (`/Game/Blueprints/Characters/BP_Digger.Dig Radius` `target digger`)) `target digger`))

(fn `Remove Speed BuffDebuff`
  (params (`speed multiplier` :type "Float (double-precision)") (`target digger` :type "/Game/Blueprints/Characters/BP_Digger Object Reference"))
  (bind _charactermovement (`Character.CharacterMovement` `target digger`))
  (set `CharacterMovementComponent.MaxWalkSpeed` (/ (`CharacterMovementComponent.MaxWalkSpeed` _charactermovement) `speed multiplier`) _charactermovement))

(fn `Return Remain BuffDebuff Data`
  (returns (`Remain BuffDebuff` :type "/Game/Blueprints/Items/S_BuffDebuffData Structure"))
  (bind (_speedmultiplier _powermultiplier _duration _deathpenalty) (break `/Game/Blueprints/Items/S_BuffDebuffData` (`self.BuffDebuff Data`)))
  (return (make `/Game/Blueprints/Items/S_BuffDebuffData` _speedmultiplier _powermultiplier (`self.GetLifeSpan`) _deathpenalty)))

(fn `Set Power BuffDebuff`
  (params (`buff debuff target` :type "/Game/Blueprints/Characters/BP_Digger Object Reference") (`power multiplier` :type "Float (double-precision)"))
  (set `/Game/Blueprints/Characters/BP_Digger.Dig Radius` (* (`/Game/Blueprints/Characters/BP_Digger.Dig Radius` `buff debuff target`) `power multiplier`) `buff debuff target`)
  (`self.SetLifeSpan` 0.0))

(fn `Set Speed BuffDebuff`
  (params (`buff debuff target` :type "/Game/Blueprints/Characters/BP_Digger Object Reference") (`speed multiplier` :type "Float (double-precision)"))
  (bind _charactermovement (`Character.CharacterMovement` `buff debuff target`))
  (set `CharacterMovementComponent.MaxWalkSpeed` (* (`CharacterMovementComponent.MaxWalkSpeed` _charactermovement) `speed multiplier`) _charactermovement))

(fn `UserConstructionScript`)