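; BP_QuickSlot holds an inventory quick slot bar as a map of index to item, with one selected index.
; Up and down selection wrap between 1 and MaxLength, returning the selected item.
; Adding refuses occupied indices; selection, add and remove changes broadcast through update dispatchers.
; Initialize stores contents and length and pads missing indices with empty entries, but never applies its SelectedIndex input.
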(fn `Add Item`
  (params (`Add Index` :type Integer) (`New Item` :type "/Game/Blueprints/Items/PDA_Item Object Reference"))
  (returns (`Add Success` :type Boolean))
  (bind _slot_contents (`self.Slot Contents`))
  (if (or (>= `Add Index` 0) (< `Add Index` (`self.Max Length`)))
    (`/Engine/EditorBlueprintResources/StandardMacros.IsValid` (`BlueprintMapLibrary.Map_Find` (`self.Slot Contents`) `Add Index`)
      (:`Is Valid`
        (`KismetSystemLibrary.PrintText` null (`|FormatText` "Already Used Index : {index}" `Add Index`))
        (return false))
      (:`Is Not Valid`
        (`BlueprintMapLibrary.Map_Add` _slot_contents `Add Index` `New Item`)
        (`self.On Slot Contents Update` _slot_contents)
        (return true)))
    (else
      (return false))))

(fn `Down Selected Index`
  (returns (`Selected Item` :type "/Game/Blueprints/Items/PDA_Item Object Reference"))
  (if (== (`self.Selected Index`) 1)
    (bind _output_get (set `self.Selected Index` (`self.Max Length`)))
    (`self.On Selected Index Update` _output_get)
    (else
      (bind _result (`/Engine/EditorBlueprintResources/StandardMacros.DecrementInt` (`self.Selected Index`))
        (:`  `
          (`self.On Selected Index Update` _result)))))
  (return (`BlueprintMapLibrary.Map_Find` (`self.Slot Contents`) (`self.Selected Index`))))

(fn `Get Selected Item`
  (returns (`Selected Item` :type "/Game/Blueprints/Items/PDA_Item Object Reference"))
  (return (`BlueprintMapLibrary.Map_Find` (`self.Slot Contents`) (`self.Selected Index`))))

(fn `Initialize`
  (params (`Slot Contents` :type "Map of Integer to /Game/Blueprints/Items/PDA_Item Object Reference") (`Max Length` :type Integer) (`Selected Index` :type Integer))
  (set `self.Slot Contents` `Slot Contents`)
  (bind _output_get (set `self.Max Length` `Max Length`))
  (for _index (range 1 (+ _output_get 1))
    (if (not (`.ReturnValue` (`BlueprintMapLibrary.Map_Find` (`self.Slot Contents`) _index)))
      (`BlueprintMapLibrary.Map_Add` (`self.Slot Contents`) _index))))

(fn `Remove Index`
  (params (`Remove Index` :type Integer))
  (bind _slot_contents (`self.Slot Contents`))
  (`BlueprintMapLibrary.Map_Remove` _slot_contents `Remove Index`)
  (`self.On Slot Contents Update` _slot_contents))

(fn `Remove Selected Item`
  (bind _slot_contents (`self.Slot Contents`))
  (`BlueprintMapLibrary.Map_Remove` _slot_contents (`self.Selected Index`))
  (`self.On Slot Contents Update` _slot_contents))

(fn `Up Selected Index`
  (returns (`Selected Item` :type "/Game/Blueprints/Items/PDA_Item Object Reference"))
  (if (== (`self.Selected Index`) (`self.Max Length`))
    (bind _output_get (set `self.Selected Index` 1))
    (`self.On Selected Index Update` _output_get)
    (else
      (bind _result (`/Engine/EditorBlueprintResources/StandardMacros.IncrementInt` (`self.Selected Index`))
        (:`  `
          (`self.On Selected Index Update` _result)))))
  (return (`BlueprintMapLibrary.Map_Find` (`self.Slot Contents`) (`self.Selected Index`))))