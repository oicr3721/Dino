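; BP_ItemInventory is an item inventory that keeps a count for each item in the Contents map.
; Add increments valid items and Subtract decrements existing ones, removing an entry only below zero, so zero-count entries remain.
; Both return success or failure, and successful changes, like Clear, broadcast the map through OnInvenUpdate.
; A MaxItemCount "inventory full" check exists but is disconnected, so capacity is not enforced.
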(fn `Add`
  (params (`New Item` :type "/Game/Blueprints/Items/PDA_Item Object Reference"))
  (returns (`Add Success` :type Boolean))
  (bind (_value _returnvalue) (`BlueprintMapLibrary.Map_Find` (`self.Contents`) `New Item`))
  (`/Engine/EditorBlueprintResources/StandardMacros.IsValid` `New Item`
    (:`Is Valid`
      (if _returnvalue
        (`BlueprintMapLibrary.Map_Add` (`self.Contents`) `New Item` (+ _value 1))
        (else
          (`BlueprintMapLibrary.Map_Add` (`self.Contents`) `New Item` 1)))
      (`self.On Inven Update` (`self.Contents`))
      (return true))
    (:`Is Not Valid`
      (return false))))

(fn `Clear`
  (bind _contents (`self.Contents`))
  (`BlueprintMapLibrary.Map_Clear` _contents)
  (`self.On Inven Update` _contents))

(fn `Subtract`
  (params (`Consume Item` :type "/Game/Blueprints/Items/PDA_Item Object Reference"))
  (returns (`Subtract Success` :type Boolean))
  (locals (`new count` :type Integer))
  (bind (_value _returnvalue) (`BlueprintMapLibrary.Map_Find` (`self.Contents`) `Consume Item`))
  (if _returnvalue
    (bind _output_get (set `local.new count` (- _value 1)))
    (`BlueprintMapLibrary.Map_Add` (`self.Contents`) `Consume Item` _output_get)
    (if (< _output_get 0)
      (`BlueprintMapLibrary.Map_Remove` (`self.Contents`) `Consume Item`))
    (`self.On Inven Update` (`self.Contents`))
    (return true)
    (else
      (return false))))