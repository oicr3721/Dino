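; BP_FossilCollection records which fossils have been registered in the collection and reports progress against all known fossils.
; Registration stores each fossil's ItemID in FossilIDCollection, which also answers whether a given fossil is already registered.
; Progress is built as an item-to-boolean map, seeding every FossilDict item as false, then flipping registered IDs that resolve through FindItem to true.
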(fn `Get Collection Progress`
  (returns (`Collection Progress` :type "Map of /Game/Blueprints/Items/PDA_Item Object Reference to Boolean"))
  (locals (`Temp Progress` :type "Map of /Game/Blueprints/Items/PDA_Item Object Reference to Boolean"))
  (for _array_element (`/Game/Blueprints/Items/PDA_ItemDict.All Items` (`self.Fossil Dict`))
    (`BlueprintMapLibrary.Map_Add` (`local.Temp Progress`) _array_element))
  (bind _valuepin (`|SetForEach` (`self.Fossil ID Collection`))
    (:`then`
      (bind (_item _find_success) (`/Game/Blueprints/Items/PDA_ItemDict.Find Item` (`self.Fossil Dict`) _valuepin))
      (if _find_success
        (`BlueprintMapLibrary.Map_Add` (`local.Temp Progress`) _item true)))
    (:`CompletedPin`
      (return (`local.Temp Progress`)))))

(fn `Is Fossil Registered`
  (params (Fossil :type "/Game/Blueprints/Items/Fossil/PDA_Fossil Object Reference"))
  (returns (`Is Registered` :type Boolean))
  (return (`BlueprintSetLibrary.Set_Contains` (`self.Fossil ID Collection`) (`/Game/Blueprints/Items/PDA_Item.Item ID` Fossil))))

(fn `Register Fossil`
  (params (`New Fossil` :type "/Game/Blueprints/Items/Fossil/PDA_Fossil Object Reference"))
  (`BlueprintSetLibrary.Set_Add` (`self.Fossil ID Collection`) (`/Game/Blueprints/Items/PDA_Item.Item ID` `New Fossil`)))