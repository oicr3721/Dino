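; BP_RockInventory is an inventory that holds rocks up to a maximum count.
; Add appends a rock only while the contents are below that limit and returns whether it succeeded.
; Clear empties the contents.
; Both successful adds and clears broadcast the updated contents through the OnInvenUpdate dispatcher, so listeners can react to changes.
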(fn `Add`
  (params (`New Rock` :type "/Game/Blueprints/Items/S_RockInfo Structure"))
  (returns (`Add Success` :type Boolean))
  (bind _contents (`self.Contents`))
  (if (< (`KismetArrayLibrary.Array_Length` (`self.Contents`)) (`self.Max Count`))
    (`KismetArrayLibrary.Array_Add` _contents `New Rock`)
    (`self.On Inven Update` _contents)
    (return true)
    (else
      (return false))))

(fn `Clear`
  (bind _contents (`self.Contents`))
  (`KismetArrayLibrary.Array_Clear` _contents)
  (`self.On Inven Update` _contents))