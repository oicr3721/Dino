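; BP_LevelTransitionManager fades the screen when a level starts and when moving to another level.
; BeginPlay plays a fade-in, while MoveToLevel plays a fade-out, waits a fixed delay, then opens the named level.
; Both use GetFadeWidget, which lazily creates a WBP_Fade widget, adds it to the viewport and caches it for reuse.
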(event `self.ReceiveBeginPlay`
  (bind _fade_widget (`self.Get Fade Widget`))
  (`/Game/Blueprints/WBP/WBP_Fade.Play Fade In` _fade_widget))

(event `Move To Level`
  (params (`Level Name` :type Name))
  (bind _fade_widget (`self.Get Fade Widget`))
  (`/Game/Blueprints/WBP/WBP_Fade.Play Fade Out` _fade_widget)
  (`KismetSystemLibrary.Delay` 1.2)
  (`GameplayStatics.OpenLevel` `Level Name`))

(fn `Get Fade Widget`
  (returns (`Fade Widget` :type "/Game/Blueprints/WBP/WBP_Fade Object Reference"))
  (bind _fade_widget (`self.Fade Widget`))
  (`/Engine/EditorBlueprintResources/StandardMacros.IsValid` _fade_widget
    (:`Is Valid`
      (return _fade_widget))
    (:`Is Not Valid`
      (bind _returnvalue (`|CreateWidget` "/Game/Blueprints/WBP/WBP_Fade.WBP_Fade_C"))
      (bind _output_get (set `self.Fade Widget` _returnvalue))
      (`UserWidget.AddToViewport` _output_get 0)
      (return _output_get))))

(fn `UserConstructionScript`)