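; BP_DiggingPoint is an interactable dig spot that yields an item after repeated digs.
; Each Interact adds to a dig count measured against a fixed requirement set at BeginPlay, with progress shown through debug prints.
; On completion it spawns a BP_WorldItem of its content type, launches it with a random upward cone impulse, and destroys itself.
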(event `self.ReceiveBeginPlay`
  (`self.SetRequiredDigs`))

(event `/Game/Blueprints/Interactions/BPI_Interact.Interact`
  (`KismetSystemLibrary.PrintString` (`KismetStringLibrary.Concat_StrStr` (`KismetSystemLibrary.GetDisplayName` self) " Interact"))
  (`self.Dug`))

(fn `Drop Item`
  (bind _returnvalue (`|SpawnActorFromClass` "/Game/Blueprints/Items/BP_WorldItem.BP_WorldItem_C" (`self.GetTransform`) "AdjustIfPossibleButAlwaysSpawn" "MultiplyWithRoot" null (`self.Content Item`) null))
  (`/Engine/EditorBlueprintResources/StandardMacros.IsValid` _returnvalue
    (:`Is Valid`
      (`PrimitiveComponent.AddImpulse` (`/Game/Blueprints/Items/BP_WorldItem.Item Mesh` _returnvalue) (* (`self.Impulse Strength`) (`KismetMathLibrary.RandomUnitVectorInConeInDegrees` (0.0 0.0 1.0) 45.0)) "None" false)
      (`KismetSystemLibrary.PrintString` "Drop Item Success"))))

(fn `Dug`
  (bind _digprogress (`self.DigProgress`))
  ; Dig Progress Update
  (set `self.DigCount` (+ (`self.DigCount`) 1))
  (set `self.DigProgress` (/ (`self.DigCount`) (`self.RequiredDigs`)))
  (if (or (`KismetMathLibrary.NearlyEqual_FloatFloat` _digprogress 1.0) (> _digprogress 1.0))
    (`self.Drop Item`)
    (`self.K2_DestroyActor`)
    (else
      ; Dig Progress Show
      (`KismetSystemLibrary.PrintString` (`KismetStringLibrary.Concat_StrStr` (`KismetStringLibrary.Conv_DoubleToString` (`self.DigProgress`)) " Dig")))))

(fn `Get Interaction Name`
  (returns (`Interaction Name` :type Text))
  (return "Dig"))

(fn `SetRequiredDigs`
  (set `self.RequiredDigs` 10)
  (`KismetSystemLibrary.PrintString` (`KismetStringLibrary.Concat_StrStr` "Required Digs " (`KismetStringLibrary.Conv_IntToString` (`self.RequiredDigs`)))))

(fn `UserConstructionScript`)