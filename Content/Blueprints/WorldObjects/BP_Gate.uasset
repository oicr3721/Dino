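; BP_Gate is an interactable world object that sends the game to the level set in its Level variable.
; Its interact event calls GoToLevel, which gets the level transition message object from the game mode and calls MoveToLevel on it.
; Two further functions, apparently interaction interface implementations, return its InteractionName and an unconditional true for any player.
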(event `Interact_1`
  (params (Player :type "/Game/Blueprints/Characters/BP_PlayerCharacter Object Reference"))
  (`self.Go To Level`))

(fn `EdGraph_4`
  (params (Player :type "/Game/Blueprints/Characters/BP_PlayerCharacter Object Reference"))
  (returns (`Interaction Name` :type Text))
  (return (`self.Interaction Name`)))

(fn `EdGraph_5`
  (params (Player :type "/Game/Blueprints/Characters/BP_PlayerCharacter Object Reference"))
  (returns (Interactable :type Boolean))
  (return true))

(fn `Go To Level`
  (bind _level_transition (message `/Game/BPI_LevelTransition.Get LevelTransition` (`GameplayStatics.GetGameMode`)))
  (`/Game/Blueprints/Managers/BP_LevelTransitionManager.Move To Level` _level_transition (`self.Level`)))

(fn `UserConstructionScript`)