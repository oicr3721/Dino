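; BP_Ladder is an interactable world object that takes the player down to the next dungeon level, shown with a "Go Down" prompt.
; On interaction it reads the current floor from GI_GameInstance and picks one of three voxel levels by floor range.
; The level change is requested through the game mode's level transition message interface, and the ladder is always interactable.
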(event `/Game/Blueprints/WorldObjects/BPI_Interact.Interact`
  (params (Player :type "/Game/Blueprints/Characters/BP_PlayerCharacter Object Reference"))
  (`self.Go Down`))

(fn `Get Interaction Name`
  (params (Player :type "/Game/Blueprints/Characters/BP_PlayerCharacter Object Reference"))
  (returns (`Interaction Name` :type Text))
  (return "Go Down"))

(fn `Go Down`
  (bind _asgi_game_instance (cast `/Game/GI_GameInstance` (`GameplayStatics.GetGameInstance`)))
  (bind _level_transition (message `/Game/BPI_LevelTransition.Get LevelTransition` (`GameplayStatics.GetGameMode`)))
  (bind _now_floor (`/Game/GI_GameInstance.Now Floor` _asgi_game_instance))
  (if (<= _now_floor 6)
    (`/Game/Blueprints/Managers/BP_LevelTransitionManager.Move To Level` _level_transition "/Game/Voxel_Theme/Lvl_Voxel1.Lvl_Voxel1")
    (elif (<= _now_floor 12)
      (`/Game/Blueprints/Managers/BP_LevelTransitionManager.Move To Level` _level_transition "/Game/Voxel_Theme/Lvl_Voxel2.Lvl_Voxel2")
      (else
        (`/Game/Blueprints/Managers/BP_LevelTransitionManager.Move To Level` _level_transition "/Game/Voxel_Theme/Lvl_Voxel3.Lvl_Voxel3")))))

(fn `Is Interactable`
  (params (Player :type "/Game/Blueprints/Characters/BP_PlayerCharacter Object Reference"))
  (returns (Interactable :type Boolean))
  (return true))

(fn `UserConstructionScript`
  (`parent.UserConstructionScript`))