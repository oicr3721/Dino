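; BP_ItemImage is a world-space item image actor that starts hidden and can be shown or hidden on demand.
; Show makes the image visible, plays a pop Actor Sequence and runs a timeline that raises a height offset.
; While visible, Tick bobs the actor on a sine wave around its start location plus that offset.
; Hide turns off visibility and resets the offset.
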(event `self.ReceiveBeginPlay`
  (set `self.Start Location` (`self.K2_GetActorLocation`))
  (set `self.Origin Scale` (`self.GetActorScale3D`))
  (`SceneComponent.SetVisibility` (`self.Item Image`) false false)
  (set `self.Plus Height` 0.0))

(event `self.ReceiveTick`
  (params (DeltaSeconds :type "Float (single-precision)"))
  (bind (_start_location_x _start_location_y _start_location_z) (`KismetMathLibrary.BreakVector` (`self.Start Location`)))
  (if (`SceneComponent.IsVisible` (`self.Item Image`))
    (bind _output_get (set `self.Running Time` (+ DeltaSeconds (`self.Running Time`))))
    (`self.K2_SetActorLocation` (`KismetMathLibrary.MakeVector` _start_location_x _start_location_y (+ (* (`KismetMathLibrary.Sin` (* _output_get (`self.Float Speed`))) (`self.Float Height`)) _start_location_z (`self.Plus Height`))))))

(event `Show`
  (`SceneComponent.SetVisibility` (`self.Item Image`) true false)
  (`ActorSequenceComponent.PlaySequence` (`self.ActorSequence_Pop`))
  (bind (_direction _timeline_float) (`Timeline|Timeline` :!via `PlayFromStart`)
    (:`Update`
      (set `self.Plus Height` (`KismetMathLibrary.Lerp` 0.0 40.0 _timeline_float)))))

(event `Hide`
  (`SceneComponent.SetVisibility` (`self.Item Image`) false false)
  (set `self.Plus Height` 0.0))

(fn `UserConstructionScript`)