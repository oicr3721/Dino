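; BP_LevelTransitionManager handles level changes with a screen fade.
; On BeginPlay it plays a fade-in after a short delay, and MoveToLevel plays a fade-out, waits, then opens the given level by object reference.
; GetFadeWidget lazily creates and caches a WBP_Fade widget and adds it to the viewport at a high Z-order.
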(event `self.ReceiveBeginPlay`
  (bind _fade_widget (`self.Get Fade Widget`))
  (`KismetSystemLibrary.Delay` 0.5)
  (`/Game/Blueprints/WBP/WBP_Fade.Play Fade In` _fade_widget))

(event `Move To Level`
  (params (Level :type "World Soft Object Reference"))
  (bind _fade_widget (`self.Get Fade Widget`))
  (`/Game/Blueprints/WBP/WBP_Fade.Play Fade Out` _fade_widget)
  (`KismetSystemLibrary.Delay` 1.0)
  (`GameplayStatics.OpenLevelBySoftObjectPtr` Level))

(fn `Get Fade Widget`
  (returns (`Fade Widget` :type "/Game/Blueprints/WBP/WBP_Fade Object Reference"))
  (bind _fade_widget (`self.Fade Widget`))
  (`/Engine/EditorBlueprintResources/StandardMacros.IsValid` _fade_widget
    (:`Is Valid`
      (return _fade_widget))
    (:`Is Not Valid`
      (bind _returnvalue (`|CreateWidget` "/Game/Blueprints/WBP/WBP_Fade.WBP_Fade_C"))
      (bind _output_get (set `self.Fade Widget` _returnvalue))
      (`UserWidget.AddToViewport` _output_get 500)
      (return _output_get))))

(fn `UserConstructionScript`)