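; Rock-breaking manager that opens the player's collected rocks one at a time on Space, or all remaining on Left Shift.
; Each rock rolls a fossil, charm or misc item from pools the construction script sorts by type and period.
; Fossil periods depend on birth floor, with luck favoring unregistered fossils.
; Fossils register and pay money, other items enter inventory, and finishing clears the rock inventory and shows a results widget.
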(event `self.ReceiveBeginPlay`
  (bind _item_image (`/Game/Blueprints/WorldObjects/BP_ItemImage.Item Image` (`self.Item Image`)))
  (bind _asgi_game_instance (cast `/Game/GI_GameInstance` (`GameplayStatics.GetGameInstance`))
    (:`then`
      (set `self.Game Instance` _asgi_game_instance)
      (bind _contents (`/Game/Blueprints/Inven/BP_RockInventory.Contents` (`/Game/GI_GameInstance.Rock Inven` _asgi_game_instance)))
      (if (> (`KismetArrayLibrary.Array_Length` _contents) 0)
        (set `self.Rocks` _contents)
        (set `self.Player Fossil Collection` (`/Game/GI_GameInstance.Fossil Collection` _asgi_game_instance))
        (`/Engine/EditorBlueprintResources/StandardMacros.IsValid` (`self.Item Image`)
          (:`Is Valid`
            _)
          (:`Is Not Valid`
            (bind _returnvalue (`|SpawnActorFromClass` "/Game/Blueprints/WorldObjects/BP_ItemImage.BP_ItemImage_C" (`self.GetTransform`) "Undefined" "MultiplyWithRoot" null null))
            (bind _output_get (set `self.Item Image` _returnvalue))
            (`SceneComponent.K2_SetWorldLocationAndRotation` (`/Game/Blueprints/WorldObjects/BP_ItemImage.Item Image` _output_get) (0.0 0.0 0.0) (struct :`Yaw` 90.0 :`Roll` 70.0) false false)))
        (bind _returnvalue_2 (`PrimitiveComponent.CreateDynamicMaterialInstance` _item_image 0 (`PrimitiveComponent.GetMaterial` _item_image 0) "None"))
        (set `self.Image Material` _returnvalue_2)
        (`self.Set Next Rock`)
        (else
          (`self.End Break Mode` :!label _label))))
    (:`CastFailed`
      (goto _label))))

(event `Set Next Rock`
  (bind _returnvalue (`self.K2_GetActorLocation`))
  (`/Game/Blueprints/WorldObjects/BP_ItemImage.Hide` (`self.Item Image`))
  (if (< (`self.Now Rock Index`) (`KismetArrayLibrary.Array_Length` (`self.Rocks`)))
    (`self.Create Breakable Rock`)
    (`/Game/Blueprints/WorldObjects/BP_BreakableRock.Move To` (`self.Now Rock`) (+ _returnvalue (0.0 0.0 400.0)) _returnvalue)
    (`KismetSystemLibrary.Delay` 1.1)
    (set `self.Can Break` true)
    (elif (not (`self.Is Skipped`))
      (`self.End Break Mode`))))

(event `Key|SpaceBar`
  (params (Key :type "Key Structure"))
  (:`Pressed`
    (if (and (`self.Can Break`) (not (`self.Is Skipped`)))
      (`self.Break Rock`))))

(event `Break Rock`
  (bind _item_image (`self.Item Image`))
  (set `self.Can Break` false)
  (bind _content (`self.Get Item` (`|GetArrayItem` (`self.Rocks`) (`self.Now Rock Index`))))
  (`/Engine/EditorBlueprintResources/StandardMacros.IncrementInt` (`self.Now Rock Index`)
    (:`  `
      (`KismetArrayLibrary.Array_Add` (`self.Result Item IDs`) (`/Game/Blueprints/Items/PDA_Item.Item ID` _content))
      (`/Game/Blueprints/WorldObjects/BP_BreakableRock.Break` (`self.Now Rock`))
      (`MaterialInstanceDynamic.SetTextureParameterValue` (`self.Image Material`) "ImageTexture" (`/Game/Blueprints/Items/PDA_Item.Item Icon` _content))
      (`/Game/Blueprints/WorldObjects/BP_ItemImage.Show` _item_image)
      (`KismetSystemLibrary.Delay` 1.5)
      (`/Game/Blueprints/WorldObjects/BP_ItemImage.Hide` _item_image)
      (`self.Set Next Rock`))))

(event `Key|LeftShift`
  (params (Key :type "Key Structure"))
  (:`Pressed`
    (if (not (`self.Is Skipped`))
      (set `self.Is Skipped` true)
      (`self.Skip Break`))))

(event `Skip Break`
  (set `self.Can Break` false)
  (for (_array_element _array_index) (`self.Rocks`)
    (if (>= _array_index (`self.Now Rock Index`))
      (bind _content (`self.Get Item` _array_element))
      (`KismetArrayLibrary.Array_Add` (`self.Result Item IDs`) (`/Game/Blueprints/Items/PDA_Item.Item ID` _content))))
  (`self.End Break Mode`))

(event `End Break Mode`
  ; Clear Rock Inven
  (bind _game_instance (`self.Game Instance`)
    (:`then`
      (`/Game/Blueprints/Inven/BP_RockInventory.Clear` (`/Game/GI_GameInstance.Rock Inven` _game_instance)))
    (:`else`
      _))
  (bind _returnvalue (`|CreateWidget` "/Game/Blueprints/WBP/WBP_BreakRockResult.WBP_BreakRockResult_C"))
  (`/Game/Blueprints/WBP/WBP_BreakRockResult.Update Result Slots` _returnvalue (`self.Result Item IDs`))
  (`UserWidget.AddToViewport` _returnvalue 0))

(fn `Create Breakable Rock`
  (bind _returnvalue (`|SpawnActorFromClass` "/Game/Blueprints/WorldObjects/BP_BreakableRock.BP_BreakableRock_C" (`SceneComponent.K2_GetComponentToWorld` (`self.DefaultSceneRoot`)) "AdjustIfPossibleButAlwaysSpawn" "MultiplyWithRoot" null null))
  (set `self.Now Rock` _returnvalue))

(fn `Get Fossil Reward`
  (params (Fossil :type "/Game/Blueprints/Items/Fossil/PDA_Fossil Object Reference"))
  (returns (Reward :type Integer))
  (locals (Multiplier :type "Float (double-precision)" :default 1.0) (`Cretaceous Reward` :type Integer :default 1000) (`Jurassic Reward` :type Integer :default 2000) (`Triassic Reward` :type Integer :default 3000))
  (if (`/Game/Blueprints/Inven/BP_FossilCollection.Is Fossil Registered` (`self.Player Fossil Collection`) Fossil)
    (set `local.Multiplier` 1.0)
    (else
      (set `local.Multiplier` 2.0)))
  (switch `/Game/Blueprints/Items/Fossil/E_FossilPeriod` (`/Game/Blueprints/Items/Fossil/PDA_Fossil.Period` Fossil)
    (:`NewEnumerator1`
      (return (`KismetMathLibrary.FTrunc` (* (`local.Multiplier`) (`local.Cretaceous Reward`)))))
    (:`NewEnumerator0`
      (return (`KismetMathLibrary.FTrunc` (* (`local.Multiplier`) (`local.Jurassic Reward`)))))
    (:`NewEnumerator2`
      (return (`KismetMathLibrary.FTrunc` (* (`local.Multiplier`) (`local.Triassic Reward`)))))))

(fn `Get Item`
  (params (`Rock Info` :type "/Game/Blueprints/Items/S_RockInfo Structure"))
  (returns (Content :type "/Game/Blueprints/Items/PDA_Item Object Reference"))
  (locals (random :type "Float (double-precision)"))
  (bind (_fossilprob _charmprob _etcprob _birthfloor) (break `/Game/Blueprints/Items/S_RockInfo` `Rock Info`))
  (bind _game_instance (`self.Game Instance`))
  (bind _output_get (set `local.random` (`KismetMathLibrary.RandomFloatInRange` 0.0 (+ (+ _fossilprob _charmprob) _etcprob))))
  (if (< _output_get _fossilprob)
    (bind _fossil (`self.Get Random Fossil` _birthfloor))
    (`/Game/Blueprints/Inven/BP_FossilCollection.Register Fossil` (`/Game/GI_GameInstance.Fossil Collection` _game_instance) _fossil)
    (bind _reward (`self.Get Fossil Reward` _fossil))
    (`/Game/GI_GameInstance.Add Player Money` _game_instance _reward)
    (return _fossil)
    (elif (< _output_get _charmprob)
      (bind _pda_charm (`self.Get Random Charms`))
      (`/Game/Blueprints/Inven/BP_ItemInventory.Add` (`/Game/GI_GameInstance.Item Inven` (`self.Game Instance`)) _pda_charm)
      (return _pda_charm)
      (else
        (bind _etc (`self.Get Random Etcs`))
        (`/Game/Blueprints/Inven/BP_ItemInventory.Add` (`/Game/GI_GameInstance.Item Inven` (`self.Game Instance`)) _etc)
        (return _etc)))))

(fn `Get Random Charms`
  (returns (`pda charm` :type "/Game/Blueprints/Items/PDA_Charm Object Reference"))
  (bind _charms (`self.Charms`))
  (return (`|GetArrayItem` _charms (`KismetMathLibrary.RandomInteger` (`KismetArrayLibrary.Array_Length` _charms)))))

(fn `Get Random Etcs`
  (returns (Etc :type "/Game/Blueprints/Items/PDA_Item Object Reference"))
  (bind _etcs (`self.Etcs`))
  (return (`|GetArrayItem` _etcs (`KismetMathLibrary.RandomInteger` (`KismetArrayLibrary.Array_Length` _etcs)))))

(fn `Get Random Fossil`
  (params (`Rock Birth Floor` :type Integer))
  (returns (Fossil :type "/Game/Blueprints/Items/Fossil/PDA_Fossil Object Reference"))
  (switch `/Game/Blueprints/Items/Fossil/E_FossilPeriod` (`self.Get Rock Period` `Rock Birth Floor`)
    (:`NewEnumerator1`
      (return (`self.Pick Fossil` (`self.Cretaceous Fossils`))))
    (:`NewEnumerator0`
      (return (`self.Pick Fossil` (`self.Jurassic Fossils`))))
    (:`NewEnumerator2`
      (return (`self.Pick Fossil` (`self.Triassic Fossils`))))))

(fn `Get Rock Period`
  (params (`Rock Birth Floor` :type Integer))
  (returns (Period :type "/Game/Blueprints/Items/Fossil/E_FossilPeriod Enum"))
  (locals (Periods :type "Array of /Game/Blueprints/Items/Fossil/E_FossilPeriod Enum"))
  (`|ExecutionSequence`
    (:`then_0`
      (if (<= `Rock Birth Floor` 10)
        (`KismetArrayLibrary.Array_AddUnique` (`local.Periods`) "NewEnumerator1"))
      (if (and (>= `Rock Birth Floor` 5) (<= `Rock Birth Floor` 15))
        (`KismetArrayLibrary.Array_AddUnique` (`local.Periods`) "NewEnumerator0"))
      (if (and (>= `Rock Birth Floor` 10) (<= `Rock Birth Floor` 20))
        (`KismetArrayLibrary.Array_AddUnique` (`local.Periods`) "NewEnumerator2")))
    (:`then_1`
      (return (`|GetArrayItem` (`local.Periods`) (`KismetMathLibrary.RandomInteger` (enumcount `/Game/Blueprints/Items/Fossil/E_FossilPeriod`)))))))

(fn `Load Dict Datas`
  (`|ExecutionSequence`
    (:`then_0`
      (for _array_element (`/Game/Blueprints/Items/PDA_ItemDict.All Items` (`self.Fossil Dict`))
        (bind _aspda_fossil (cast `/Game/Blueprints/Items/Fossil/PDA_Fossil` _array_element))
        (switch `/Game/Blueprints/Items/Fossil/E_FossilPeriod` (`/Game/Blueprints/Items/Fossil/PDA_Fossil.Period` _aspda_fossil)
          (:`NewEnumerator1`
            (`KismetArrayLibrary.Array_AddUnique` (`self.Cretaceous Fossils`) _aspda_fossil))
          (:`NewEnumerator0`
            (`KismetArrayLibrary.Array_AddUnique` (`self.Jurassic Fossils`) _aspda_fossil))
          (:`NewEnumerator2`
            (`KismetArrayLibrary.Array_AddUnique` (`self.Triassic Fossils`) _aspda_fossil)))))
    (:`then_1`
      (for _array_element_2 (`/Game/Blueprints/Items/PDA_ItemDict.All Items` (`self.Item Dict`))
        (bind _aspda_charm (cast `/Game/Blueprints/Items/PDA_Charm` _array_element_2)
          (:`then`
            (`KismetArrayLibrary.Array_AddUnique` (`self.Charms`) _aspda_charm))
          (:`CastFailed`
            (cast `/Game/Blueprints/Items/PDA_Food` _array_element_2
              (:`CastFailed`
                (cast `/Game/Blueprints/Items/PDA_Shovel` _array_element_2
                  (:`CastFailed`
                    (`KismetArrayLibrary.Array_AddUnique` (`self.Etcs`) _array_element_2)))))))))))

(fn `Pick Fossil`
  (params (Fossils :type "Array of /Game/Blueprints/Items/Fossil/PDA_Fossil Object Reference"))
  (returns (Fossil :type "/Game/Blueprints/Items/Fossil/PDA_Fossil Object Reference"))
  (locals (`Fossil Probs Array` :type "Array of Float (double-precision)") (`Base Prob` :type "Float (double-precision)" :default 1.0) (`Max Prob Temp` :type "Float (double-precision)") (Random :type "Float (double-precision)") (`Prob Temp` :type "Float (double-precision)"))
  (bind _base_prob (`local.Base Prob`))
  (bind _returnvalue (+ (`local.Base Prob`) (`self.Player Luck`)))
  (for _array_element Fossils
    (if (`/Game/Blueprints/Inven/BP_FossilCollection.Is Fossil Registered` (`self.Player Fossil Collection`) _array_element)
      (`KismetArrayLibrary.Array_Add` (`local.Fossil Probs Array`) _base_prob)
      (set `local.Max Prob Temp` (+ _base_prob (`local.Max Prob Temp`)))
      (else
        (`KismetArrayLibrary.Array_Add` (`local.Fossil Probs Array`) _returnvalue)
        (set `local.Max Prob Temp` (+ _returnvalue (`local.Max Prob Temp`))))))
  (set `local.Random` (`KismetMathLibrary.RandomFloatInRange` 0.0 (`local.Max Prob Temp`)))
  (for (_array_element_2 _array_index) (`local.Fossil Probs Array`)
    (set `local.Prob Temp` (+ (`local.Prob Temp`) _array_element_2))
    (if (< (`local.Random`) (`local.Prob Temp`))
      (return (`|GetArrayItem` Fossils _array_index))))
  (return "/Game/Blueprints/Items/Fossil/FDA_Pteranodon.FDA_Pteranodon"))

(fn `UserConstructionScript`
  (`self.Load Dict Datas`))