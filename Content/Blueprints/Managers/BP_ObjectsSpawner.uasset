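; Level manager that procedurally scatters fabric props, rocks and ladders across the current floor on BeginPlay.
; Fabric goes first as random child-actor variants at Poisson-like points, with a sphere trace to replace rocks and avoid ladders.
; A second point set guarantees one ladder, then rolls luck-based ladder odds per point, otherwise spawning rocks.
; Rocks get randomized visuals and loot odds, with fossil chance scaled by floor and dino luck.
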(event `self.ReceiveBeginPlay`
  (bind _asgi_game_instance (cast `/Game/GI_GameInstance` (`GameplayStatics.GetGameInstance`)))
  (set `self.GI` _asgi_game_instance)
  (`self.Generate Fabric`)
  (`self.Generate Rocks And Ladders`))

(fn `Generate Fabric`
  (bind _returnvalue (`PointDistributionLibrary.GeneratePoissonLikePoints` (-700.0 -700.0) (700.0 700.0) 300.0 5 200 0.0 (`KismetMathLibrary.RandomInteger` 1000000)))
  (for _array_element _returnvalue
    (bind _outhit (`KismetSystemLibrary.SphereTraceSingle` _array_element _array_element 100.0 "TraceTypeQuery1"))
    (bind (_bblockinghit _binitialoverlap _time _distance _location _impactpoint _normal _impactnormal _physmat _hitactor) (`GameplayStatics.BreakHitResult` _outhit))
    (bind _asbp_rock (cast `/Game/Blueprints/Items/BP_Rock` _hitactor)
      (:`then`
        (`self.K2_DestroyActor` _asbp_rock))
      (:`CastFailed`
        (cast `/Game/Blueprints/WorldObjects/BP_Ladder` _hitactor
          (:`CastFailed`
            _))))
    (bind _returnvalue_2 (`AddComponent|NODE_AddChildActorComponent-2` :`RelativeTransform` (`KismetMathLibrary.Conv_VectorToTransform` _array_element)))
    (`ChildActorComponent.SetChildActorClass` _returnvalue_2 (select `int` (`KismetMathLibrary.RandomIntegerInRange` 0 3) :`0` "/Game/Blueprints/WorldObjects/Fabric/BP_FabricA.BP_FabricA_C" :`1` "/Game/Blueprints/WorldObjects/Fabric/BP_FabricB.BP_FabricB_C" :`2` "/Game/Blueprints/WorldObjects/Fabric/BP_FabricC.BP_FabricC_C" :`3` "/Game/Blueprints/WorldObjects/Fabric/BP_FabricD.BP_FabricD_C" :!type "Actor Class Reference"))))

(fn `Generate Rock Info`
  (returns (`New Rock Info` :type "/Game/Blueprints/Items/S_RockInfo Structure"))
  (bind _returnvalue (`KismetMathLibrary.RandomFloatInRange` 0.85 1.15))
  (bind _gi (`self.GI`))
  (bind _now_floor (`/Game/GI_GameInstance.Now Floor` _gi))
  (bind (_key _value) (`BlueprintMapLibrary.Map_GetKeyValueByIndex` (`self.Rock Visual`) (`KismetMathLibrary.RandomIntegerInRange` 0 (- (`BlueprintMapLibrary.Map_Length` (`self.Rock Visual`)) 1))))
  (return (make `/Game/Blueprints/Items/S_RockInfo` (* (+ (`/Game/GI_GameInstance.Get Dino Luck` _gi) (`KismetMathLibrary.SafeDivide` (`KismetMathLibrary.Conv_IntToDouble` _now_floor) 10.0)) _returnvalue) (* _returnvalue 0.4) (* _returnvalue 0.5) _now_floor _key _value)))

(fn `Generate Rocks And Ladders`
  (locals (`Confirmed Ladder Index` :type Integer))
  (bind _returnvalue (`PointDistributionLibrary.GeneratePoissonLikePoints` (-700.0 -700.0) (700.0 700.0) (`self.Min Distance`) 30 30 -50.0 (`KismetMathLibrary.RandomInteger` 1000000)))
  (set `local.Confirmed Ladder Index` (`KismetMathLibrary.RandomInteger` (`KismetArrayLibrary.Array_Length` _returnvalue)))
  (`|SpawnActorFromClass` "/Game/Blueprints/WorldObjects/BP_Ladder.BP_Ladder_C" (`KismetMathLibrary.Conv_VectorToTransform` (`|GetArrayItem` _returnvalue (`local.Confirmed Ladder Index`))) "AlwaysSpawn" "MultiplyWithRoot" null null)
  (`KismetArrayLibrary.Array_Remove` _returnvalue (`local.Confirmed Ladder Index`))
  (for _array_element _returnvalue
    (if (`self.Is Ladder`)
      (bind _returnvalue_2 (`KismetMathLibrary.Conv_VectorToTransform` _array_element))
      (`|SpawnActorFromClass` "/Game/Blueprints/WorldObjects/BP_Ladder.BP_Ladder_C" _returnvalue_2 "AlwaysSpawn" "MultiplyWithRoot" null null)
      (else
        (`|SpawnActorFromClass` "/Game/Blueprints/Items/BP_Rock.BP_Rock_C" _returnvalue_2 "AlwaysSpawn" "MultiplyWithRoot" null (`self.Generate Rock Info`) null)))))

(fn `Get Charm Prob`
  (params (`Ladder Prob` :type "Float (double-precision)") (`Dino Prob` :type "Float (double-precision)"))
  (returns (`Charm Prob` :type "Float (double-precision)"))
  (return (* (- 1.0 (+ `Ladder Prob` `Dino Prob`)) 0.02)))

(fn `Get Dino Prob`
  (params (`Current Floor` :type Integer))
  (returns (`Dino Prob` :type "Float (double-precision)"))
  (bind _asgi_game_instance (cast `/Game/GI_GameInstance` (`GameplayStatics.GetGameInstance`))
    (:`then`
      (return (* (+ (/ `Current Floor` 10) (`/Game/GI_GameInstance.Get Dino Luck` _asgi_game_instance)) 0.05)))
    (:`CastFailed`
      (return 0.0))))

(fn `Get Ladder Prob`
  (returns (`Ladder Prob` :type "Float (double-precision)"))
  (bind _asgi_game_instance (cast `/Game/GI_GameInstance` (`GameplayStatics.GetGameInstance`))
    (:`then`
      (return (* (+ 1.0 (`/Game/GI_GameInstance.Get Ladder Luck` _asgi_game_instance)) 0.05)))
    (:`CastFailed`
      (return 0.0))))

(fn `Is Ladder`
  (returns (`Is Ladder` :type Boolean))
  (locals (rand :type "Float (double-precision)") (`dino prob` :type "Float (double-precision)") (`ladder prob` :type "Float (double-precision)"))
  (set `local.rand` (`KismetMathLibrary.RandomFloatInRange` 0.0 1.0))
  (set `local.ladder prob` (`self.Get Ladder Prob`))
  (if (< (`local.rand`) (`local.ladder prob`))
    (return true)
    (else
      (return false))))

(fn `UserConstructionScript`)