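; BP_ItemSpawner is a manager that scatters buried items and "Go Down" ladders over a square area on BeginPlay.
; It generates Poisson-like spaced points, then picks a type for each using luck values from GI_GameInstance.
; Fossil, Food, Rock and Other all currently spawn the same fossil item, while Charm has no spawn branch.
; If no ladder spawns, a fallback adds one at a random item's location and destroys a randomly indexed item.
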(event `self.ReceiveBeginPlay`
  (bind _items (`self.Items`))
  (bind _output (`|GetArrayItem` _items (`KismetMathLibrary.RandomIntegerInRange` 0 (- (`KismetArrayLibrary.Array_Length` _items) 1))))
  (bind _returnvalue (`PointDistributionLibrary.GeneratePoissonLikePoints` (-500.0 -500.0) (500.0 500.0) (`self.Min Distance`) 30 30 -50.0))
  (for _array_element _returnvalue
    (bind _item_type (`self.SelectItemType`))
    (switch `/Game/Blueprints/Items/E_ItemType` _item_type
      (:`NewEnumerator0`
        (bind _returnvalue_2 (`|SpawnActorFromClass` "/Game/Blueprints/Items/BP_ItemInTheGround.BP_ItemInTheGround_C" (`KismetMathLibrary.Conv_VectorToTransform` _array_element) "AlwaysSpawn" "MultiplyWithRoot" null "/Game/Blueprints/Items/IDA_Fossil_1.IDA_Fossil_1" null :!label _label))
        (`/Engine/EditorBlueprintResources/StandardMacros.IsValid` _returnvalue_2
          (:`Is Valid`
            (`KismetArrayLibrary.Array_Add` (`self.Items`) _returnvalue_2))))
      (:`NewEnumerator1`
        (goto _label))
      (:`NewEnumerator2`
        (goto _label))
      (:`NewEnumerator3`
        (`|SpawnActorFromClass` "/Game/Blueprints/Objects/BP_Ladder.BP_Ladder_C" (`KismetMathLibrary.Conv_VectorToTransform` _array_element) "AlwaysSpawn" "MultiplyWithRoot" null "Lvl_Voxel" "Go Down" null)
        (set `self.ladder count` (+ 1 (`self.ladder count`)))
        (`KismetSystemLibrary.PrintString` "Spawn Ladder"))
      (:`NewEnumerator4`
        (goto _label))))
  (if (< (`self.ladder count`) 1)
    (`|SpawnActorFromClass` "/Game/Blueprints/Objects/BP_Ladder.BP_Ladder_C" (`KismetMathLibrary.Conv_VectorToTransform` (`self.K2_GetActorLocation` _output)) "AlwaysSpawn" "MultiplyWithRoot" null "Lvl_Voxel" "Go Down" null)
    (`self.K2_DestroyActor` _output)
    (`KismetSystemLibrary.PrintString` "Replace Item With Ladder")))

(fn `Get Charm Prob`
  (params (`Ladder Prob` :type "Float (double-precision)") (`Dino Prob` :type "Float (double-precision)"))
  (returns (`Charm Prob` :type "Float (double-precision)"))
  (return (* (- 1.0 (+ `Ladder Prob` `Dino Prob`)) 0.02)))

(fn `Get Dino Prob`
  (params (`Current Floor` :type Integer))
  (returns (`Dino Prob` :type "Float (double-precision)"))
  (bind _asgi_game_instance (cast `/Game/GI_GameInstance` (`GameplayStatics.GetGameInstance`))
    (:`then`
      (return (* (+ (/ `Current Floor` 10) (`/Game/GI_GameInstance.Get Dino Luck` _asgi_game_instance)) 0.05)))
    (:`CastFailed`
      (return 0.0))))

(fn `Get Ladder Prob`
  (returns (`Ladder Prob` :type "Float (double-precision)"))
  (bind _asgi_game_instance (cast `/Game/GI_GameInstance` (`GameplayStatics.GetGameInstance`))
    (:`then`
      (return (* (+ 1.0 (`/Game/GI_GameInstance.Get Ladder Luck` _asgi_game_instance)) 0.05)))
    (:`CastFailed`
      (return 0.0))))

(fn `SelectItemType`
  (returns (`Item Type` :type "/Game/Blueprints/Items/E_ItemType Enum"))
  (locals (rand :type "Float (double-precision)") (`dino prob` :type "Float (double-precision)") (`ladder prob` :type "Float (double-precision)"))
  (set `local.rand` (`KismetMathLibrary.RandomFloatInRange` 0.0 1.0))
  (set `local.dino prob` (`self.Get Dino Prob` 1))
  (set `local.ladder prob` (`self.Get Ladder Prob`))
  (if (< (`local.dino prob`) (`local.rand`))
    (return "NewEnumerator0")
    (elif (< (`local.ladder prob`) (`local.rand`))
      (return "NewEnumerator3")
      (elif (> (`self.Get Charm Prob` (`local.ladder prob`) (`local.dino prob`)) (`local.rand`))
        (return "NewEnumerator5")
        (else
          (return "NewEnumerator4"))))))

(fn `UserConstructionScript`)