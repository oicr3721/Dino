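; BP_Dad is an interactable character named "Dad" who breaks the player's rocks when interacted with.
; BreakRocks loops over the GI_GameInstance rock inventory, rolling a random number against each rock's Fossil, Charm and Etc weights.
; The Charm check compares against its own weight rather than a cumulative total, skewing the odds.
; Results are only printed; the inventory is left unchanged.
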(event `/Game/Blueprints/Objects/BPI_Interact.Interact`
  (params (Player :type "/Game/Blueprints/Characters/BP_PlayerCharacter Object Reference"))
  (`self.Break Rocks`))

(fn `Break Rocks`
  (locals (`random float` :type "Float (double-precision)"))
  (bind _asgi_game_instance (cast `/Game/GI_GameInstance` (`GameplayStatics.GetGameInstance`)))
  (for _array_element (`/Game/Blueprints/Inven/BP_RockInventory.Contents` (`/Game/GI_GameInstance.Rock Inven` _asgi_game_instance))
    (bind (_fossilprob _charmprob _etcprob) (break `/Game/Blueprints/Items/S_RockInfo` _array_element))
    (set `local.random float` (`KismetMathLibrary.RandomFloatInRange` 0.0 (+ (+ _fossilprob _charmprob) _etcprob)))
    (if (< (`local.random float`) _fossilprob)
      (`KismetSystemLibrary.PrintString` "Fossil")
      (elif (< (`local.random float`) _charmprob)
        (`KismetSystemLibrary.PrintString` "Charm")
        (else
          (`KismetSystemLibrary.PrintString` "Etc"))))))

(fn `Get Interaction Name`
  (params (Player :type "/Game/Blueprints/Characters/BP_PlayerCharacter Object Reference"))
  (returns (`Interaction Name` :type Text))
  (return "Dad"))

(fn `Is Interactable`
  (params (Player :type "/Game/Blueprints/Characters/BP_PlayerCharacter Object Reference"))
  (returns (Interactable :type Boolean))
  (return true))

(fn `UserConstructionScript`)