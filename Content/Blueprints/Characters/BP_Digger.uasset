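; BP_Digger is a character that digs into voxel terrain and can carry attached BP_BuffDebuff actors.
; TraceDigPoint sphere-traces from the capsule toward a forward point with negated world Z, returning a point sunk into the hit VoxelWorld.
; StartDig waits DigDuration, carves and smooths a sphere there, fires Niagara effects, then clears IsDigging.
; ApplyPenalty is an empty stub, and nothing here calls the trace.
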(event `self.ReceiveBeginPlay`
  (set `CharacterMovementComponent.MaxWalkSpeed` (`self.Base Speed`) (`self.CharacterMovement`)))

(event `Start Dig`
  (params (`Dig Point` :type "Vector Structure") (`Voxel World` :type "VoxelWorld Object Reference"))
  (set `self.Is Digging` true)
  (`KismetSystemLibrary.Delay` (`self.Dig Duration`))
  (`self.Dig Voxel` `Dig Point` `Voxel World`)
  (`self.Excute Dig`))

(fn `Apply Penalty`)

(fn `Attach Buff Debuff`
  (params (BuffDebuffData :type "/Game/Blueprints/Items/S_BuffDebuffData Structure"))
  (bind _returnvalue (`|SpawnActorFromClass` "/Game/Blueprints/Items/BP_BuffDebuff.BP_BuffDebuff_C" (`KismetMathLibrary.MakeTransform` (0.0 0.0 0.0)) "AlwaysSpawn" "MultiplyWithRoot" null BuffDebuffData null))
  (`self.K2_AttachToActor` _returnvalue self "None" "KeepRelative" "KeepRelative" "KeepRelative" true))

(fn `Dig Voxel`
  (params (`Dig Point` :type "Vector Structure") (`Voxel World` :type "VoxelWorld Object Reference"))
  (bind _niagara (`self.Niagara`))
  (`VoxelSphereTools.RemoveSphere` `Voxel World` `Dig Point` (`self.Dig Radius`))
  (`VoxelSphereTools.SmoothSphere` `Voxel World` `Dig Point` (* (`self.Dig Radius`) 1.5) 70.0 1 "Tip")
  (`SceneComponent.K2_SetWorldLocation` _niagara `Dig Point` false false)
  (`ActorComponent.Activate` _niagara true))

(fn `Excute Dig`
  (set `self.Is Digging` false))

(fn `Get Trace End Pos`
  (returns (pos :type "Vector Structure"))
  (bind _capsulecomponent (`self.CapsuleComponent`))
  (return (* (+ (`SceneComponent.K2_GetComponentLocation` _capsulecomponent) (* (`SceneComponent.GetForwardVector` _capsulecomponent) (`self.Dig Distance`))) (1.0 1.0 -1.0))))

(fn `Get Trace Start Pos`
  (returns (pos :type "Vector Structure"))
  (return (`SceneComponent.K2_GetComponentLocation` (`self.CapsuleComponent`))))

(fn `Trace Dig Point`
  (returns (`Dig Point` :type "Vector Structure") (`Voxel World` :type "VoxelWorld Object Reference") (Success :type Boolean))
  (bind _outhit (`KismetSystemLibrary.SphereTraceSingle` :`Start` (`self.Get Trace Start Pos`) :`End` (`self.Get Trace End Pos`) :`Radius` 10.0 :`TraceChannel` "TraceTypeQuery3" :`DrawTime` 2.0))
  (bind (_bblockinghit _binitialoverlap _time _distance _location _impactpoint _normal _impactnormal _physmat _hitactor) (`GameplayStatics.BreakHitResult` _outhit))
  (bind _asvoxel_world (cast `VoxelWorld` _hitactor)
    (:`then`
      (return (- _impactpoint (* _normal (`self.Dig Depth`))) _asvoxel_world true))
    (:`CastFailed`
      (return (0.0 0.0 0.0) null false))))

(fn `UserConstructionScript`)