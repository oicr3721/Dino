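; Behavior tree service that sets an AI pawn's dig destination from the DigTarget blackboard actor when the service activates.
; If the pawn's 2D distance to the target exceeds MinDistance, it writes the target's location to the selected key.
; Otherwise it writes an away-from-target offset vector scaled by DesiredDistance minus current distance, without adding a world position.
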(event `self.ReceiveActivationAI`
  (params (OwnerController :type "AIController Object Reference") (ControlledPawn :type "Pawn Object Reference"))
  (bind _returnvalue (`Actor.K2_GetActorLocation` ControlledPawn))
  (`KismetSystemLibrary.PrintString` "Dig Destination_BT Service")
  (bind _asactor (cast `Actor` (`BlackboardComponent.GetValueAsObject` (`AIBlueprintHelperLibrary.GetBlackboard` OwnerController) "DigTarget")))
  (bind _returnvalue_2 (`Actor.K2_GetActorLocation` _asactor))
  (bind _returnvalue_3 (`KismetMathLibrary.Vector_Distance2D` _returnvalue _returnvalue_2))
  (if (> _returnvalue_3 (`self.Min Distance`))
    (`BTFunctionLibrary.SetBlackboardValueAsVector` (`self.BlackboardKey`) _returnvalue_2)
    (else
      (`BTFunctionLibrary.SetBlackboardValueAsVector` (`self.BlackboardKey`) (* (- (`self.Desired Distance`) _returnvalue_3) (`KismetMathLibrary.Normal` (- _returnvalue _returnvalue_2) 0.1))))))