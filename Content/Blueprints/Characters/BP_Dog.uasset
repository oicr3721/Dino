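; Dog companion that follows the player, digs toward nearby rocks and can be fed food for buffs or debuffs.
; An AIMoveTo-driven event loop alternates following with sphere-overlap searches for BP_Rock, then traces a voxel-world dig point and retries after each dig.
; Active effects are restored from the GameInstance on BeginPlay and saved on EndPlay.
; The death penalty destroys the dog and clears HasDog.
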(event `self.ReceiveBeginPlay`
  ; Attach Remain Buff or Debuff
  (bind _asgi_game_instance (cast `/Game/GI_GameInstance` (`GameplayStatics.GetGameInstance`)))
  (for _array_element (`/Game/GI_GameInstance.Dog Active Effects` _asgi_game_instance)
    (`self.Attach Buff Debuff` _array_element)
    (`self.K2_SetActorLocation` (`self.K2_GetActorLocation`) true))
  (`self.Follow Player`))

(event `Move To Dig`
  (`KismetSystemLibrary.PrintString` "Move To Dig")
  (`/Engine/EditorBlueprintResources/StandardMacros.IsValid` (`self.Dig Target`)
    (:`Is Valid`
      (`|AIMoveTo` self (`self.Get Dig Destination`) null 20.0
        (:`OnSuccess`
          _)
        (:`OnFail`
          _))
      (`self.Try Dig`))
    (:`Is Not Valid`
      (`self.Follow Player`))))

(event `Follow Player`
  (`KismetSystemLibrary.PrintString` "Follow Player")
  (`|AIMoveTo` self (0.0 0.0 0.0) (`GameplayStatics.GetPlayerCharacter` 0) 100.0
    (:`OnSuccess`
      (`KismetSystemLibrary.Delay` 2.0)
      (if (`KismetMathLibrary.RandomBool`)
        (`self.Find Dig Target` :!label _label)
        (else
          (`self.Follow Player`))))
    (:`OnFail`
      (goto _label))))

(event `Try Dig`
  (bind _dig_target (`self.Dig Target`))
  (bind _returnvalue (`self.GetDistanceTo` _dig_target))
  (`/Engine/EditorBlueprintResources/StandardMacros.IsValid` _dig_target
    (:`Is Valid`
      (`KismetSystemLibrary.PrintText` (`|FormatText` "Try Dig {Target}" _dig_target))
      (if (< _returnvalue 20.0)
        (`KismetSystemLibrary.PrintText` (`|FormatText` "Dig Complete : distance {dist}" _returnvalue))
        (`self.Follow Player`)
        (else
          (bind (_dig_point _voxel_world _success) (`self.Trace Dig Point`))
          (if _success
            (`self.Start Dig` _dig_point _voxel_world)
            (else
              (`self.Follow Player`))))))
    (:`Is Not Valid`
      (`KismetSystemLibrary.PrintString` "Dig Target is not valid")
      (`self.Follow Player`))))

(event `/Game/Blueprints/Objects/BPI_Interact.Interact`
  (params (Player :type "/Game/Blueprints/Characters/BP_PlayerCharacter Object Reference"))
  (bind _selected_item (`/Game/Blueprints/Characters/BP_PlayerCharacter.Selected Item` Player))
  (bind _aspda_food (cast `/Game/Blueprints/Items/PDA_Food` _selected_item)
    (:`then`
      (`self.Attach Buff Debuff` (`.DogBuffDebuff_32_B531E6664417DA3C9A8A8685017E438D` (break `/Game/Blueprints/Items/S_ItemEffect` (`/Game/Blueprints/Items/PDA_Food.Stat Modifier` _aspda_food))))
      (`KismetSystemLibrary.PrintString` (`KismetTextLibrary.Conv_TextToString` (`|FormatText` "Dog Eat {Food}" (`/Game/Blueprints/Items/PDA_Item.Item Name` _selected_item))))
      (`/Game/Blueprints/Inven/BP_QuickSlot.Remove Selected Item` (`/Game/Blueprints/Characters/BP_PlayerCharacter.Quick Slot` Player)))
    (:`CastFailed`
      (`KismetSystemLibrary.PrintString` "Dog is happy!"))))

(event `self.ReceiveEndPlay`
  (params (EndPlayReason :type "EEndPlayReason Enum" :default "Destroyed"))
  (bind _asgi_game_instance (cast `/Game/GI_GameInstance` (`GameplayStatics.GetGameInstance`)))
  (`/Game/GI_GameInstance.Save Dog Buff Debuff` _asgi_game_instance (`self.Active BuffDebuffs`)))

(fn `Apply Penalty`
  (`KismetSystemLibrary.PrintString` "Dead : Buff Penalty")
  (`self.K2_DestroyActor`)
  (bind _asgi_game_instance (cast `/Game/GI_GameInstance` (`GameplayStatics.GetGameInstance`)))
  (set `/Game/GI_GameInstance.Has Dog` false _asgi_game_instance))

(fn `End Dig`
  (`self.Try Dig`))

(fn `Find Dig Target`
  (bind (_outactors _returnvalue) (`KismetSystemLibrary.SphereOverlapActors` (`SceneComponent.K2_GetComponentLocation` (`self.Mesh`)) 200.0 (`|MakeArray` "ObjectTypeQuery2" :!type "EObjectTypeQuery Enum") "/Game/Blueprints/Items/BP_Rock.BP_Rock_C"))
  (if _returnvalue
    (for _array_element _outactors
      (bind _asbp_rock (cast `/Game/Blueprints/Items/BP_Rock` _array_element))
      (`/Engine/EditorBlueprintResources/StandardMacros.IsValid` _asbp_rock
        (:`Is Valid`
          (set `self.Dig Target` _asbp_rock)
          (break))
        (:`Is Not Valid`
          (set `self.Dig Target` _asbp_rock))))
    (`self.Move To Dig`)
    (else
      (set `self.Dig Target` null)
      (`self.Follow Player`))))

(fn `Get Dig Destination`
  (returns (Destination :type "Vector Structure"))
  (locals (`Min Distance` :type "Float (double-precision)" :default 15.0) (`Desired Distance` :type "Float (double-precision)" :default 20.0))
  (bind _returnvalue (`self.K2_GetActorLocation`))
  (bind _returnvalue_2 (`self.K2_GetActorLocation` (`self.Dig Target`)))
  (bind _returnvalue_3 (`KismetMathLibrary.Vector_Distance2D` _returnvalue _returnvalue_2))
  (if (> _returnvalue_3 (`local.Min Distance`))
    (return _returnvalue_2)
    (else
      (return (* (- (`local.Desired Distance`) _returnvalue_3) (`KismetMathLibrary.Normal` (- _returnvalue _returnvalue_2) 0.1))))))

(fn `Get Interaction Name`
  (params (Player :type "/Game/Blueprints/Characters/BP_PlayerCharacter Object Reference"))
  (returns (`Interaction Name` :type Text))
  (`/Engine/EditorBlueprintResources/StandardMacros.IsValid` Player
    (:`Is Valid`
      (bind _aspda_food (cast `/Game/Blueprints/Items/PDA_Food` (`/Game/Blueprints/Characters/BP_PlayerCharacter.Selected Item` Player))
        (:`then`
          (return (`|FormatText` "Feed {Food}" (`/Game/Blueprints/Items/PDA_Item.Item Name` _aspda_food))))
        (:`CastFailed`
          (return "Good Boy"))))))

(fn `Is Interactable`
  (params (Player :type "/Game/Blueprints/Characters/BP_PlayerCharacter Object Reference"))
  (returns (Interactable :type Boolean))
  (return true))

(fn `UserConstructionScript`)